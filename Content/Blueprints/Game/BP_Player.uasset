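; Player Blueprint that gives visual feedback for the Slam and SuperCharge inputs by changing the mesh material and point light.
; SuperCharge swaps to a brighter light-blue look while held, sets a Charging flag, and restores the default blue on release.
; Slam flashes a red look, then reverts after a short delay unless Charging is set.
; No movement or ability logic is here, and a velocity debug print is left unconnected.
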(event Custom|Set%20Defaults)

(event EventBeginPlay)

(event Collision|EventActorBeginOverlap
  (params (OtherActor :type Actor%20Object%20Reference)))

(event Input|ActionEvents|InputActionSuperCharge
  (params (Key :type Key%20Structure :default "None"))
  (:Pressed
    (Rendering|Material|SetMaterial (Variables|Character|GetMesh) 0 "/Game/Materials/MAT_Player_inst.MAT_Player_inst")
    (Variables|Default|SetCharging true)
    (Rendering|Components|Light|SetIntensity (Variables|Default|GetPointLight) 5e+02)
    (Rendering|Components|Light|SetLightColor (Variables|Default|GetPointLight) "(R=0.060764,G=0.415256,B=0.729167,A=1.000000)" true))
  (:Released
    (Rendering|Material|SetMaterial (Variables|Character|GetMesh) 0 "/Game/Materials/MAT_Player.MAT_Player")
    (Variables|Default|SetCharging false)
    (Rendering|Components|Light|SetIntensity (Variables|Default|GetPointLight) 1e+02)
    (Rendering|Components|Light|SetLightColor (Variables|Default|GetPointLight) "(R=0.000000,G=0.070352,B=0.729167,A=1.000000)" true)))

(event Input|ActionEvents|InputActionSlam
  (params (Key :type Key%20Structure :default "None"))
  (:Pressed
    (Rendering|Material|SetMaterial (Variables|Character|GetMesh) 0 "/Game/Materials/MAT_Player_inst2.MAT_Player_inst2")
    (Rendering|Components|Light|SetLightColor (Variables|Default|GetPointLight) "(R=0.729167,G=0.007596,B=0.007596,A=1.000000)" true)
    (Utilities|FlowControl|Delay 0.4)
    (if (not (Variables|Default|GetCharging))
      (Rendering|Material|SetMaterial (Variables|Character|GetMesh) 0 "/Game/Materials/MAT_Player.MAT_Player")
      (Rendering|Components|Light|SetLightColor (Variables|Default|GetPointLight) "(R=0.000000,G=0.070352,B=0.729167,A=1.000000)" true)
      (Rendering|Components|Light|SetIntensity (Variables|Default|GetPointLight) 1e+02))))

(fn ConstructionScript)