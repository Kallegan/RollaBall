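; Game mode base that runs a time-of-day clock for the level's BP_CustomSunSky.
; On BeginPlay it finds the sky actor and starts a looping timer at the AmountToTickSeconds interval.
; Each tick advances DayTimeSeconds and writes its timespan hours, minutes and seconds to the sky.
; At 86400 seconds it zeroes AmountToTickSeconds, without resetting DayTimeSeconds or the running timer.
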(event Custom|TimeUpdate
  (bind _sun_sky (Variables|Default|GetSun%20Sky))
  (bind _output_get (Variables|Default|SetDayTimeSeconds (+ (Variables|Default|GetDayTimeSeconds) (Variables|Default|GetAmountOfSecondsToAddTick))))
  (Variables|/Game/Sky/BP_CustomSunSky.BP_CustomSunSky_C|SetHours _sun_sky (.Hours (Math|Timespan|BreakTimespan (Math|Timespan|MakeTimespan 0 0 0 _output_get))))
  (Variables|/Game/Sky/BP_CustomSunSky.BP_CustomSunSky_C|SetMinutes _sun_sky (.Minutes (Math|Timespan|BreakTimespan (Math|Timespan|MakeTimespan 0 0 0 _output_get))))
  (Variables|/Game/Sky/BP_CustomSunSky.BP_CustomSunSky_C|SetSeconds _sun_sky (.Seconds (Math|Timespan|BreakTimespan (Math|Timespan|MakeTimespan 0 0 0 _output_get))))
  (if (>= (Variables|Default|GetDayTimeSeconds) 86400)
    (Variables|Default|SetAmountToTickSeconds 0.0)))

(event EventBeginPlay
  (bind _returnvalue (Actor|GetActorOfClass "/Game/Sky/BP_CustomSunSky.BP_CustomSunSky_C"))
  (bind _asbp_custom_sun_sky (Utilities|Casting|CastToBP_CustomSunSky _returnvalue))
  (Variables|Default|SetSun%20Sky _asbp_custom_sun_sky)
  (Utilities|Time|SetTimerbyEvent (delegate Custom|TimeUpdate) (/ (Variables|Default|GetAmountToTickSeconds) 1.0) true))

(fn ConstructionScript)