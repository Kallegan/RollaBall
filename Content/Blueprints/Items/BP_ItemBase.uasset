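; BP_ItemBase is a collectible item base Blueprint that plays a short effect when collected, then removes itself.
; The Collected event runs once, calls the parent implementation and speeds up the RotatingMovement yaw spin tenfold.
; It spawns the AttributeReaderTrails particle system at the item's location, then destroys that effect and the actor after a brief delay.
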(event EventBeginPlay)

(event Collision|EventActorBeginOverlap
  (params (OtherActor :type Actor%20Object%20Reference)))

(event EventCollected
  (Utilities|FlowControl|DoOnce false
    (:Completed
      (|CallParentFunction)
      (Variables|/Script/Engine.RotatingMovementComponent|SetRotationRate (Variables|Default|GetRotatingMovement) (Math|Rotator|MakeRotator 0.0 0.0 (* 1e+01 (.yaw (Variables|/Script/Engine.RotatingMovementComponent|GetRotationRate (Variables|Default|GetRotatingMovement))))))
      (bind _returnvalue (Niagara|SpawnSystematLocation "/Niagara/DefaultAssets/Templates/Systems/AttributeReaderTrails.AttributeReaderTrails" (Transformation|GetActorLocation) "0, 0, 0" "2.000000,2.000000,2.000000"))
      (Utilities|FlowControl|Delay 0.5)
      (Components|DestroyComponent _returnvalue)
      (Actor|DestroyActor))))

(fn ConstructionScript)