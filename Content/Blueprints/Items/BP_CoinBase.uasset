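; BP_CoinBase is a coin item that handles its own collection feedback and removal.
; Its Collected event runs only once through a DoOnce, calls the parent implementation, then zeroes the RotatingMovement rotation rate to stop the spin.
; It spawns a scaled-up SimpleExplosion Niagara effect at the coin's location, then destroys both the effect and the actor after a short delay.
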(event EventBeginPlay)

(event Collision|EventActorBeginOverlap
  (params (OtherActor :type Actor%20Object%20Reference)))

(event EventTick
  (params (DeltaSeconds :type Float%20%28single-precision%29)))

(event EventCollected
  (Utilities|FlowControl|DoOnce false
    (:Completed
      (|CallParentFunction)
      (Variables|/Script/Engine.RotatingMovementComponent|SetRotationRate (Variables|Default|GetRotatingMovement) (Math|Rotator|MakeRotator 0.0 0.0 (* (.yaw (Variables|/Script/Engine.RotatingMovementComponent|GetRotationRate (Variables|Default|GetRotatingMovement))) 0.0)))
      (bind _returnvalue (Niagara|SpawnSystematLocation "/Niagara/DefaultAssets/Templates/Systems/SimpleExplosion.SimpleExplosion" (Transformation|GetActorLocation) "0, 0, 0" "2.000000,2.000000,2.000000"))
      (Utilities|FlowControl|Delay 0.5)
      (Components|DestroyComponent _returnvalue)
      (Actor|DestroyActor))))

(fn ConstructionScript)